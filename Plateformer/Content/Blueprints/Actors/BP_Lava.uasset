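; BP_Lava is a rising lava hazard that resets the level's progress when the player touches its box.
; Tick interpolates the mesh upward, and the Start event enables ticking after a delay if GonnaMove is set.
; BeginPlay caches the player's and lava's start transforms, the key and all collectibles.
; On overlap it stops ticking, restores those positions, zeroes score, decrements the key count, re-shows the pickups and calls Start again.
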(event OnComponentBeginOverlap(Box)
  (params (OverlappedComponent :type Primitive%20Component%20Object%20Reference) (OtherActor :type Actor%20Object%20Reference) (OtherComp :type Primitive%20Component%20Object%20Reference) (OtherBodyIndex :type Integer) (bFromSweep :type Boolean) (SweepResult :type Hit%20Result%20Structure%20%28by%20ref%29))
  (bind _keyref (Variables|Default|GetKeyRef))
  (bind _asbp_third_person_character (Utilities|Casting|CastToBP_ThirdPersonCharacter OtherActor))
  (Actor|Tick|SetActorTickEnabled false)
  (Transformation|SetActorLocation (Variables|Default|GetLavaLocation) false false)
  (Variables|/Game/ThirdPerson/Blueprints/BP_ThirdPersonCharacter.BP_ThirdPersonCharacter_C|SetScore _asbp_third_person_character 0)
  (Math|Integer|DecrementInt (Variables|/Game/ThirdPerson/Blueprints/BP_ThirdPersonCharacter.BP_ThirdPersonCharacter_C|GetNbrKey _asbp_third_person_character)
    (:%20%20
      (Transformation|SetActorLocationAndRotation _asbp_third_person_character (Variables|Default|GetPlayerLocation) (Variables|Default|GetPlayerRotation))
      (Rendering|SetActorHiddenInGame _keyref false)
      (Collision|SetActorEnableCollision _keyref true)
      (for _array_element (Variables|Default|GetCollectibles)
        (Rendering|SetActorHiddenInGame _array_element false)
        (Collision|SetActorEnableCollision _array_element true))
      (CallFunction|Start))))

(event Custom|Start
  (Utilities|FlowControl|Delay 1e+01)
  (if (Variables|Default|GetGonnaMove)
    (Actor|Tick|SetActorTickEnabled true)))

(event EventBeginPlay
  (bind _asbp_third_person_character (Utilities|Casting|CastToBP_ThirdPersonCharacter (Game|GetPlayerCharacter 0)))
  (Variables|Default|SetPlayerLocation (Transformation|GetActorLocation _asbp_third_person_character))
  (Variables|Default|SetPlayerRotation (Transformation|GetActorRotation _asbp_third_person_character))
  (Variables|Default|SetLavaLocation (Transformation|GetActorLocation))
  (bind _outactors (Actor|GetAllActorsOfClass "/Game/Blueprints/Actors/BP_Collectible.BP_Collectible_C"))
  (Variables|Default|SetCollectibles _outactors)
  (bind _returnvalue (Actor|GetActorOfClass "/Game/Blueprints/Actors/BP_Key.BP_Key_C"))
  (Variables|Default|SetKeyRef _returnvalue))

(event Collision|EventActorBeginOverlap
  (params (OtherActor :type Actor%20Object%20Reference)))

(event EventTick
  (params (DeltaSeconds :type Float%20%28single-precision%29))
  (bind _staticmeshcomponent (Variables|Debug|GetStaticMeshComponent))
  (bind _relativelocation (Variables|/Script/Engine.SceneComponent|GetRelativeLocation _staticmeshcomponent))
  (bind (_x _y _z) (Math|Vector|BreakVector _relativelocation))
  (Transformation|SetRelativeLocation _staticmeshcomponent (Math|Interpolation|VInterpTo _relativelocation (Math|Vector|MakeVector _x _y (+ _z 4e+01)) DeltaSeconds 3.0) false false))

(fn ConstructionScript)