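; BP_Bumper is an interactive actor that acts as either a launching bumper or a disappearing trap, depending on its Trap flag.
; On Interaction, a normal bumper launches the cached player character along its forward vector scaled by Force, overriding Z velocity.
; A trap instead runs a timeline that slides it a short world-Y offset from its start.
; It then hides and drops collision briefly before restoring both.
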(event EventBeginPlay
  (bind _returnvalue (Transformation|GetActorLocation))
  (bind _asbp_third_person_character (Utilities|Casting|CastToBP_ThirdPersonCharacter (Game|GetPlayerCharacter 0)))
  (Variables|Default|SetPlayerRef _asbp_third_person_character)
  (Variables|Default|SetStartLocation _returnvalue)
  (Variables|Default|SetEndLocation (+ _returnvalue (Math|Vector|MakeVector 0.0 2e+01 0.0))))

(event Collision|EventActorBeginOverlap
  (params (OtherActor :type Actor%20Object%20Reference)))

(event EventTick
  (params (DeltaSeconds :type Float%20%28single-precision%29)))

(event EventInteraction
  (if (not (Variables|Default|GetTrap))
    (Character|LaunchCharacter (Variables|Default|GetPlayerRef) (* (Transformation|GetActorForwardVector) (Variables|Default|GetForce)) false true)
    (else
      (bind _move (Timeline|Timeline PlayFromStart)
        (:Update
          (Transformation|SetActorLocation (Math|Vector|Lerp(Vector) (Variables|Default|GetStartLocation) (Variables|Default|GetEndLocation) _move) false false))
        (:Finished
          (Collision|SetActorEnableCollision false)
          (Rendering|SetActorHiddenInGame true)
          (Utilities|FlowControl|Delay 2.0)
          (Collision|SetActorEnableCollision true)
          (Rendering|SetActorHiddenInGame false))))))

(fn ConstructionScript)