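; BP_Wind is a wind volume actor that pushes the third-person player character along the actor's up vector while inside its box.
; On box overlap it stores the character and starts a fast looping timer that calls Fly.
; Fly repeatedly launches the character by Force, overriding only Z velocity, so rotating the actor redirects the push.
; Leaving the box clears the timer and the stored reference.
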(event OnComponentBeginOverlap(Box)
  (params (OverlappedComponent :type Primitive%20Component%20Object%20Reference) (OtherActor :type Actor%20Object%20Reference) (OtherComp :type Primitive%20Component%20Object%20Reference) (OtherBodyIndex :type Integer) (bFromSweep :type Boolean) (SweepResult :type Hit%20Result%20Structure%20%28by%20ref%29))
  (bind _asbp_third_person_character (Utilities|Casting|CastToBP_ThirdPersonCharacter OtherActor))
  (Variables|Default|SetPlayerRef _asbp_third_person_character)
  (bind _returnvalue (Utilities|Time|SetTimerbyEvent (delegate Custom|Fly) 0.05 true))
  (Variables|Default|SetTimer _returnvalue))

(event OnComponentEndOverlap(Box)
  (params (OverlappedComponent :type Primitive%20Component%20Object%20Reference) (OtherActor :type Actor%20Object%20Reference) (OtherComp :type Primitive%20Component%20Object%20Reference) (OtherBodyIndex :type Integer))
  (Utilities|Casting|CastToBP_ThirdPersonCharacter OtherActor)
  (Utilities|Time|ClearandInvalidateTimerbyHandle (Variables|Default|GetTimer))
  (Variables|Default|SetPlayerRef 0))

(event Custom|Fly
  (Character|LaunchCharacter (Variables|Default|GetPlayerRef) (* (Transformation|GetActorUpVector) (Variables|Default|GetForce)) false true))

(event EventBeginPlay)

(event Collision|EventActorBeginOverlap
  (params (OtherActor :type Actor%20Object%20Reference)))

(fn ConstructionScript)