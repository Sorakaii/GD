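; BP_CloseFloor is an actor that slides two floor pieces in opposite directions along the Y axis when MoveFloor is triggered.
; BeginPlay caches each floor's world location and computes fixed offset end positions.
; MoveFloor plays a timeline whose Move track lerps both floors from start to end without sweeping.
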(event Custom|MoveFloor
  (bind _move (Timeline|Timeline PlayFromStart)
    (:Update
      (Transformation|SetWorldLocation (Variables|Default|GetFloor1) (Math|Vector|Lerp(Vector) (Variables|Default|GetF1BaseLocation) (Variables|Default|GetF1EndLocation) _move) false false)
      (Transformation|SetWorldLocation (Variables|Default|GetFloor2) (Math|Vector|Lerp(Vector) (Variables|Default|GetF2BaseLocation) (Variables|Default|GetF2EndLocation) _move) false false))))

(event EventBeginPlay
  (Variables|Default|SetF1BaseLocation (Transformation|GetWorldLocation (Variables|Default|GetFloor1)))
  (Variables|Default|SetF2BaseLocation (Transformation|GetWorldLocation (Variables|Default|GetFloor2)))
  (Variables|Default|SetF1EndLocation (- (Variables|Default|GetF1BaseLocation) "0.000000,2160.000000,0.000000"))
  (Variables|Default|SetF2EndLocation (+ (Variables|Default|GetF2BaseLocation) "0.000000,2000.000000,0.000000")))

(event Collision|EventActorBeginOverlap
  (params (OtherActor :type Actor%20Object%20Reference)))

(event EventTick
  (params (DeltaSeconds :type Float%20%28single-precision%29)))

(fn ConstructionScript)