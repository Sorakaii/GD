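; BP_WaterPack is an interactable pickup actor that gives the player a water pack and respawns after a short delay.
; It caches the player as BP_ThirdPersonCharacter on BeginPlay.
; Its Interaction event sets HasWaterPack on the player, calls TimerWaterPack there, then hides the mesh and disables its collision.
; A one-shot timer fires Update to restore visibility and collision, reusing the actor instead of destroying it.
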(event Custom|Update
  (bind _waterpack (Variables|Default|GetWaterPack))
  (Collision|SetCollisionEnabled _waterpack "QueryAndPhysics")
  (Rendering|SetVisibility _waterpack true false))

(event EventBeginPlay
  (bind _asbp_third_person_character (Utilities|Casting|CastToBP_ThirdPersonCharacter (Game|GetPlayerCharacter 0)))
  (Variables|Default|SetPlayerRef _asbp_third_person_character))

(event Collision|EventActorBeginOverlap
  (params (OtherActor :type Actor%20Object%20Reference)))

(event EventTick
  (params (DeltaSeconds :type Float%20%28single-precision%29)))

(event EventInteraction
  (bind _waterpack (Variables|Default|GetWaterPack))
  (Variables|/Game/ThirdPerson/Blueprints/BP_ThirdPersonCharacter.BP_ThirdPersonCharacter_C|SetHasWaterPack (Variables|Default|GetPlayerRef) true)
  (Collision|SetCollisionEnabled _waterpack "NoCollision")
  (Rendering|SetVisibility _waterpack false false)
  (Utilities|Time|SetTimerbyEvent (delegate Custom|Update) 1e+01)
  (Default|TimerWaterPack (Variables|Default|GetPlayerRef)))

(fn ConstructionScript)