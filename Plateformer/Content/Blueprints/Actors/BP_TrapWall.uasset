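; Trap wall actor that springs when the third-person character enters its trigger box, then advances as a moving wall.
; The overlap calls TrapEvent on the character, destroys the box and plays a rate-adjustable timeline lerping the wall mesh's Z toward HauteurZ.
; When the timeline finishes, it enables Tick and sets player walk speed to 1200.
; Tick interpolates toward an offset from the current position, so the wall keeps sliding along relative Y.
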(event OnComponentBeginOverlap(Box)
  (params (OverlappedComponent :type Primitive%20Component%20Object%20Reference) (OtherActor :type Actor%20Object%20Reference) (OtherComp :type Primitive%20Component%20Object%20Reference) (OtherBodyIndex :type Integer) (bFromSweep :type Boolean) (SweepResult :type Hit%20Result%20Structure%20%28by%20ref%29))
  (bind _staticmeshcomponent5 (Variables|Default|GetStaticMeshComponent5))
  (bind _relativelocation (Variables|/Script/Engine.SceneComponent|GetRelativeLocation _staticmeshcomponent5))
  (bind (_x _y) (Math|Vector|BreakVector _relativelocation))
  (bind _asbp_third_person_character (Utilities|Casting|CastToBP_ThirdPersonCharacter OtherActor))
  (Default|TrapEvent _asbp_third_person_character)
  (Components|DestroyComponent (Variables|Default|GetBox))
  (Components|Timeline|SetPlayRate (Variables|Default|GetTimeline) (Variables|Default|GetTimeLineRate))
  (bind _move (Timeline|Timeline PlayFromStart)
    (:Update
      (Transformation|SetRelativeLocation _staticmeshcomponent5 (Math|Vector|Lerp(Vector) _relativelocation (Math|Vector|MakeVector _x _y (Variables|Default|GetHauteurZ)) _move) false false))
    (:Finished
      (Actor|Tick|SetActorTickEnabled true)
      (Variables|/Script/Engine.CharacterMovementComponent|SetMaxWalkSpeed (Variables|/Script/Engine.Character|GetCharacterMovement (Variables|Default|GetPlayerRef)) 1.2e+03))))

(event EventBeginPlay
  (bind _asbp_third_person_character (Utilities|Casting|CastToBP_ThirdPersonCharacter (Game|GetPlayerCharacter 0)))
  (Variables|Default|SetPlayerRef _asbp_third_person_character))

(event EventTick
  (params (DeltaSeconds :type Float%20%28single-precision%29))
  (bind _staticmeshcomponent5 (Variables|Default|GetStaticMeshComponent5))
  (bind _relativelocation (Variables|/Script/Engine.SceneComponent|GetRelativeLocation _staticmeshcomponent5))
  (bind (_x _y _z) (Math|Vector|BreakVector _relativelocation))
  (Transformation|SetRelativeLocation _staticmeshcomponent5 (Math|Interpolation|VInterpTo _relativelocation (Math|Vector|MakeVector _x (+ _y 4.4e+02) _z) DeltaSeconds 3.0) false false))

(fn ConstructionScript)