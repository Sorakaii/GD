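; BP_Fire is a fire trap actor that hits the player with a timed burst of flame when its trigger box is overlapped.
; Any overlap swaps the Window material, then a one-second delay leads to a second swap and the activation of NSFire.
; A damage box is created at runtime in front of the actor, calling EventHit on any BP_ThirdPersonCharacter that begins overlapping it.
; Three seconds later the box is destroyed, the fire deactivates and the material changes again.
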(event OnComponentBeginOverlap(Box)
  (params (OverlappedComponent :type Primitive%20Component%20Object%20Reference) (OtherActor :type Actor%20Object%20Reference) (OtherComp :type Primitive%20Component%20Object%20Reference) (OtherBodyIndex :type Integer) (bFromSweep :type Boolean) (SweepResult :type Hit%20Result%20Structure%20%28by%20ref%29))
  (Rendering|Material|SetMaterial (Variables|Default|GetWindow) 0 "/Game/ScienceLab/Materials/ScientificDevice/MI_ScientificDevice02.MI_ScientificDevice02")
  (Utilities|FlowControl|Delay 1.0)
  (Rendering|Material|SetMaterial (Variables|Default|GetWindow) 0 "/Game/ScienceLab/Materials/ScientificDevice/MI_ScientificDevice04.MI_ScientificDevice04")
  (bind _returnvalue (AddComponent|AddBoxComponent false (Math|Transform|MakeTransform "600.000000,0.000000,0.000000" "0, 0, 0" "1.000000,1.000000,1.000000")))
  (bind _output_get (Variables|Default|SetBoxCollision _returnvalue))
  (Development|SetHiddeninGame _output_get false false)
  (Collision|BindEventtoOnComponentBeginOverlap _output_get (delegate Custom|BindedOverlap))
  (Transformation|SetRelativeLocation _output_get "600.000000,0.000000,0.000000" false false)
  (Components|Box|SetBoxExtent _output_get "600.000000,100.000000,30.000000" true)
  (Components|Activation|Activate (Variables|Default|GetNS_Fire) false)
  (Utilities|FlowControl|Delay 3.0)
  (Rendering|Material|SetMaterial (Variables|Default|GetWindow) 0 "/Game/ScienceLab/Materials/ScientificDevice/MI_GasCylinder03.MI_GasCylinder03")
  (Components|DestroyComponent (Variables|Default|GetBoxCollision))
  (Components|Activation|Deactivate (Variables|Default|GetNS_Fire)))

(event Custom|BindedOverlap
  (params (OverlappedComponent :type Primitive%20Component%20Object%20Reference) (OtherActor :type Actor%20Object%20Reference) (OtherComp :type Primitive%20Component%20Object%20Reference) (OtherBodyIndex :type Integer) (bFromSweep :type Boolean) (SweepResult :type Hit%20Result%20Structure%20%28by%20ref%29))
  (bind _asbp_third_person_character (Utilities|Casting|CastToBP_ThirdPersonCharacter OtherActor))
  (Default|EventHit _asbp_third_person_character))

(event EventBeginPlay)

(fn ConstructionScript)