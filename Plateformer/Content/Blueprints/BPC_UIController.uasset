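; UI controller Blueprint that shows the WBP_Menu widget and handles gamepad input for it.
; On BeginPlay it creates the menu, stores it in MenuRef and adds it to the viewport.
; D-pad left and right both call the menu's Move with no direction argument.
; The bottom face button presses ButtonSelected when InMenu is true and that reference, set by the menu widget, is valid.
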(event EventBeginPlay
  (bind _returnvalue (UserInterface|CreateWidget "/Game/Blueprints/UI/WBP_Menu.WBP_Menu_C"))
  (bind _output_get (Variables|Default|SetMenuRef _returnvalue))
  (UserInterface|Viewport|AddtoViewport _output_get 0))

(event EventTick
  (params (DeltaSeconds :type Float%20%28single-precision%29)))

(event Input|GamepadEvents|GamepadFaceButtonBottom
  (params (Key :type Key%20Structure :default "None"))
  (:Pressed
    (if (Variables|Default|GetInMenu)
      (bind _buttonselected (Variables|Default|GetButtonSelected) ; a set au begin du widget du menu
        (:then
          (Default|Press _buttonselected))
        (:else)))))

(event Input|GamepadEvents|GamepadDPadRight
  (params (Key :type Key%20Structure :default "None"))
  (:Pressed
    (Default|Move+ (Variables|Default|GetMenuRef))))

(event Input|GamepadEvents|GamepadDPadLeft
  (params (Key :type Key%20Structure :default "None"))
  (:Pressed
    (Default|Move- (Variables|Default|GetMenuRef))))

(fn ConstructionScript)