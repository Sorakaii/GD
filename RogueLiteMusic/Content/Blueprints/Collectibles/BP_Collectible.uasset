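; BP_Collectible is a music-genre pickup that the third-person character collects by touching it.
; The construction script picks the sphere's material from its Type, so each genre has its own look.
; On collision overlap with BP_ThirdPersonCharacter, it adds to that character's count for the Type, puts a new WBP_BoonHUD for that type on the viewport, then destroys itself.
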(event OnComponentBeginOverlap(Collision)
  (params (OverlappedComponent :type Primitive%20Component%20Object%20Reference) (OtherActor :type Actor%20Object%20Reference) (OtherComp :type Primitive%20Component%20Object%20Reference) (OtherBodyIndex :type Integer) (bFromSweep :type Boolean) (SweepResult :type Hit%20Result%20Structure%20%28by%20ref%29))
  (bind _asbp_third_person_character (Utilities|Casting|CastToBP_ThirdPersonCharacter OtherActor))
  (Default|AddCount _asbp_third_person_character (Variables|Default|GetType))
  (bind _returnvalue (UserInterface|CreateWidget "/Game/Blueprints/Widget/WBP_BoonHUD.WBP_BoonHUD_C" 0 (Variables|Default|GetType)))
  (UserInterface|Viewport|AddtoViewport _returnvalue 0)
  (Actor|DestroyActor))

(event EventBeginPlay)

(event Collision|EventActorBeginOverlap
  (params (OtherActor :type Actor%20Object%20Reference)))

(event EventTick
  (params (DeltaSeconds :type Float%20%28single-precision%29)))

(fn ConstructionScript
  (Rendering|Material|SetMaterial (Variables|Default|GetSphere) 0 (Utilities|Select :Index (Variables|Default|GetType) :NewEnumerator0 "/Game/Materials/M_Rock.M_Rock" :NewEnumerator1 "/Game/Materials/M_Pop.M_Pop" :NewEnumerator2 "/Game/Materials/M_Jazz.M_Jazz" :NewEnumerator3 "/Game/Materials/M_Classic.M_Classic" :NewEnumerator4 "/Game/Materials/M_Electro.M_Electro" :NewEnumerator5 "/Game/Materials/M_Country.M_Country")))