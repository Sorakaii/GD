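; BP_EnviroSpawner places environment actors themed by music genre at preset spawn points.
; BeginPlay gathers three spawn components into an array.
; Each SpawnEnviro call creates a BP_Enviro at the current point's world location, sets its mesh material from the genre type, then advances the index.
; The index has no wrap or bounds check here.
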(event Custom|SpawnEnviro
  (params (Type :type E_CollectibleType%20Enum :default "NewEnumerator0"))
  (bind _returnvalue (Game|SpawnActorfromClass "/Game/Blueprints/DynamicEnviro/BP_Enviro.BP_Enviro_C" (Math|Transform|MakeTransform (Transformation|GetWorldLocation (Utilities|Array|Get(acopy) (Variables|Default|GetSpawnArray) (Variables|Default|GetIndex))) "0, 0, 0" "1.000000,1.000000,1.000000") "Undefined" "MultiplyWithRoot" 0 0))
  (Rendering|Material|SetMaterial (Variables|/Game/Blueprints/DynamicEnviro/BP_Enviro.BP_Enviro_C|GetStaticMesh _returnvalue) 0 (Utilities|Select :Index Type :NewEnumerator0 "/Game/Materials/M_Rock.M_Rock" :NewEnumerator1 "/Game/Materials/M_Pop.M_Pop" :NewEnumerator2 "/Game/Materials/M_Jazz.M_Jazz" :NewEnumerator3 "/Game/Materials/M_Classic.M_Classic" :NewEnumerator4 "/Game/Materials/M_Electro.M_Electro" :NewEnumerator5 "/Game/Materials/M_Country.M_Country"))
  (Math|Integer|IncrementInt (Variables|Default|GetIndex)))

(event EventBeginPlay
  (Variables|Default|SetSpawnArray (Utilities|Array|MakeArray (Variables|Default|GetSpawn1) (Variables|Default|GetSpawn2) (Variables|Default|GetSpawn3))))

(event Collision|EventActorBeginOverlap
  (params (OtherActor :type Actor%20Object%20Reference)))

(event EventTick
  (params (DeltaSeconds :type Float%20%28single-precision%29)))

(fn ConstructionScript)