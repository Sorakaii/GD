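; Blueprint function library with shared helpers for cards: widget movement and random card selection.
; InterpolateTowardPosition eases a widget transform's translation and angle toward a destination using delta-time interpolation, without carrying over scale or shear.
; GetRandomCard switches on card type (Warrior, Wizard or Rogue) and returns a random row from that class's parameter data table.
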(fn InterpolateTowardPosition
  (params (CurrentPosition :type Widget%20Transform%20Structure) (DestinationTransform :type Widget%20Transform%20Structure) (Delta :type Float%20%28double-precision%29) (InterpolateSpeed :type Float%20%28double-precision%29))
  (bind (_translation _scale _shear _angle) (Utilities|Struct|BreakWidgetTransform DestinationTransform))
  (bind (_translation_2 _scale_2 _shear_2 _angle_2) (Utilities|Struct|BreakWidgetTransform CurrentPosition))
  (return (Utilities|Struct|MakeWidgetTransform (Class|KismetMathLibrary|Vector2DInterpto _translation_2 _translation Delta InterpolateSpeed) "(X=1.000000,Y=1.000000)" "(X=0.000000,Y=0.000000)" (Math|Interpolation|FInterpTo _angle_2 _angle Delta InterpolateSpeed))))

(fn GetRandomCard
  (params (CardType :type E_CharacterCard%20Enum :default "NewEnumerator0"))
  (switch Utilities|FlowControl|Switch|SwitchonE_CharacterCard CardType
    (:NewEnumerator0
      (bind _outrownames (DataTable|GetDataTableRowNames "/Game/Blueprints/Tuto/DT_CardParamWarrior.DT_CardParamWarrior"))
      (bind _returnvalue (Utilities|GetDataTableRow "/Game/Blueprints/Tuto/DT_CardParamWarrior.DT_CardParamWarrior" (.OutItem (Utilities|Array|Random _outrownames)))
        (:then
          (LocalVariables|SetParamOut _returnvalue)
          (return (LocalVariables|GetParamOut)))
        (:RowNotFound
          _)))
    (:NewEnumerator1
      (bind _outrownames_2 (DataTable|GetDataTableRowNames "/Game/Blueprints/Tuto/DT_CardParamWizard.DT_CardParamWizard"))
      (bind _returnvalue_2 (Utilities|GetDataTableRow "/Game/Blueprints/Tuto/DT_CardParamWizard.DT_CardParamWizard" (.OutItem (Utilities|Array|Random _outrownames_2)))
        (:then
          (LocalVariables|SetParamOut _returnvalue_2)
          (return (LocalVariables|GetParamOut)))
        (:RowNotFound
          _)))
    (:NewEnumerator2
      (bind _outrownames_3 (DataTable|GetDataTableRowNames "/Game/Blueprints/Tuto/DT_CardParamRogue.DT_CardParamRogue"))
      (bind _returnvalue_3 (Utilities|GetDataTableRow "/Game/Blueprints/Tuto/DT_CardParamRogue.DT_CardParamRogue" (.OutItem (Utilities|Array|Random _outrownames_3)))
        (:then
          (LocalVariables|SetParamOut _returnvalue_3)
          (return (LocalVariables|GetParamOut)))
        (:RowNotFound
          _))))
  (return ""))