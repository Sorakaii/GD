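; BPF_Utility is a Blueprint utility for neighbor lookups on an integer 2D grid.
; ClampIntPoint returns a point lying between zero and GridSize inclusive, otherwise a -999 sentinel rather than a clamped value.
; GetNeighbor passes the eight surrounding cells through that check and filters out sentinels by X.
; The AddUnique step that would collect valid neighbors is disconnected, so the function returns no results.
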(fn ClampIntPoint
  (params (input :type Int%20Point%20Structure) (GridSize :type Int%20Point%20Structure))
  (if (Math|Boolean|ANDBoolean (<= (.x input) (.x GridSize)) (<= (.y input) (.y GridSize)) (> (.x input) -1) (> (.y input) -1))
    (return input)
    (else
      (return (Utilities|Struct|MakeIntPoint -999 -999)))))

(fn GetNeighbor
  (params (Index :type Int%20Point%20Structure) (GridSize :type Int%20Point%20Structure))
  (for _array_element (Utilities|Array|MakeArray (CallFunction|ClampIntPoint (+ Index (Utilities|Struct|MakeIntPoint 1 0)) GridSize) (CallFunction|ClampIntPoint (+ Index (Utilities|Struct|MakeIntPoint 1 1)) GridSize) (CallFunction|ClampIntPoint (+ Index (Utilities|Struct|MakeIntPoint 1 -1)) GridSize) (CallFunction|ClampIntPoint (+ Index (Utilities|Struct|MakeIntPoint -1 0)) GridSize) (CallFunction|ClampIntPoint (+ Index (Utilities|Struct|MakeIntPoint -1 1)) GridSize) (CallFunction|ClampIntPoint (+ Index (Utilities|Struct|MakeIntPoint -1 -1)) GridSize) (CallFunction|ClampIntPoint (+ Index (Utilities|Struct|MakeIntPoint 0 1)) GridSize) (CallFunction|ClampIntPoint (+ Index (Utilities|Struct|MakeIntPoint 0 -1)) GridSize))
    (if (!= (.X (Utilities|Struct|BreakIntPoint _array_element)) -999)
      _))
  (return 0))