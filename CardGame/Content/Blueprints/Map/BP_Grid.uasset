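; Grid actor that moves its Pawn component at random between five linked cells, Case1 to Case5.
; BeginPlay stores the cells in Path and starts a looping one-second timer on Movement.
; Movement prints the current Index, rolls one of four directions and, if that link exists, snaps Pawn to the new cell's relative X/Y.
; Links are hard-coded index checks: a line from Case1 to Case3, which branches to Case4 and Case5.
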(event Custom|Movement
  (Development|PrintString (Utilities|String|ToString(Integer) (Variables|Default|GetIndex)))
  (switch int (Math|Random|RandomIntegerinRange 0 3)
    (:0
      (if (<= (Variables|Default|GetIndex) 1)
        (Math|Integer|IncrementInt (Variables|Default|GetIndex)
          (:%20%20
            (Transformation|SetRelativeLocation (Variables|Default|GetPawn) (Math|Vector|MakeVector (.x (Variables|/Script/Engine.SceneComponent|GetRelativeLocation (Utilities|Array|Get(acopy) (Variables|Default|GetPath) (Variables|Default|GetIndex)))) (.y (Variables|/Script/Engine.SceneComponent|GetRelativeLocation (Utilities|Array|Get(acopy) (Variables|Default|GetPath) (Variables|Default|GetIndex)))) 0.0) false false)))))
    (:1
      (if (and (<= (Variables|Default|GetIndex) 2) (> (Variables|Default|GetIndex) 0))
        (Math|Integer|DecrementInt (Variables|Default|GetIndex)
          (:%20%20
            (Transformation|SetRelativeLocation (Variables|Default|GetPawn) (Math|Vector|MakeVector (.x (Variables|/Script/Engine.SceneComponent|GetRelativeLocation (Utilities|Array|Get(acopy) (Variables|Default|GetPath) (Variables|Default|GetIndex)))) (.y (Variables|/Script/Engine.SceneComponent|GetRelativeLocation (Utilities|Array|Get(acopy) (Variables|Default|GetPath) (Variables|Default|GetIndex)))) 0.0) false false)))))
    (:2
      (switch int (Variables|Default|GetIndex)
        (:2
          (Variables|Default|SetIndex 4))
        (:3
          (Variables|Default|SetIndex 2)))
      (Transformation|SetRelativeLocation (Variables|Default|GetPawn) (Math|Vector|MakeVector (.x (Variables|/Script/Engine.SceneComponent|GetRelativeLocation (Utilities|Array|Get(acopy) (Variables|Default|GetPath) (Variables|Default|GetIndex)))) (.y (Variables|/Script/Engine.SceneComponent|GetRelativeLocation (Utilities|Array|Get(acopy) (Variables|Default|GetPath) (Variables|Default|GetIndex)))) 0.0) false false))
    (:3
      (switch int (Variables|Default|GetIndex)
        (:2
          (Variables|Default|SetIndex 3))
        (:4
          (Variables|Default|SetIndex 2)))
      (Transformation|SetRelativeLocation (Variables|Default|GetPawn) (Math|Vector|MakeVector (.x (Variables|/Script/Engine.SceneComponent|GetRelativeLocation (Utilities|Array|Get(acopy) (Variables|Default|GetPath) (Variables|Default|GetIndex)))) (.y (Variables|/Script/Engine.SceneComponent|GetRelativeLocation (Utilities|Array|Get(acopy) (Variables|Default|GetPath) (Variables|Default|GetIndex)))) 0.0) false false))))

(event EventBeginPlay
  (Variables|Default|SetPath (Utilities|Array|MakeArray (Variables|Default|GetCase1) (Variables|Default|GetCase2) (Variables|Default|GetCase3) (Variables|Default|GetCase4) (Variables|Default|GetCase5)))
  (Utilities|Time|SetTimerbyEvent (delegate Custom|Movement) 1.0 true))

(event Collision|EventActorBeginOverlap
  (params (OtherActor :type Actor%20Object%20Reference)))

(event EventTick
  (params (DeltaSeconds :type Float%20%28single-precision%29)))

(fn ConstructionScript)