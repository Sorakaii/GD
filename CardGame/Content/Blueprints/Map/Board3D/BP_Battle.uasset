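; Battle board actor that builds a 3D grid of frames on BeginPlay and seeds it with enemy cards.
; Nested loops spawn attached BP_Frames, storing column frames by coordinate in GridIndex; each row's anchor frame stays out of the map.
; AddCards randomly samples that map, placing up to three BP_Cards on empty frames in the first two Y indices.
; Tick prints every grid key as debug output.
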(event Custom|AddCards
  ;[1 0 0] Add enemies in grid
  (bind _keys (Utilities|Map|Keys (Variables|Grid|GetGridIndex)))
  (for _array_element _keys
    (bind _values (Utilities|Map|Values (Variables|Grid|GetGridIndex)))
    (bind _output_get (Variables|Default|SetFrameCard (.OutItem (Utilities|Array|Random _values))))
    (Variables|Default|SetFrameSelected (.Frame (Utilities|Struct|BreakSTR_CardPosition _output_get)))
    (if (and (< (.y (.Index (Utilities|Struct|BreakSTR_CardPosition _output_get))) 2) (<= (Variables|Default|GetNbrEnemies) 2))
      (if (Variables|/Game/Blueprints/Map/Board3D/BP_Frame.BP_Frame_C|GetIsEmpty (Variables|Default|GetFrameSelected))
        (bind _returnvalue (Game|SpawnActorfromClass "/Game/Blueprints/Map/Board3D/BP_Card.BP_Card_C" (Math|Transform|MakeTransform (Transformation|GetActorLocation (Variables|Default|GetFrameSelected)) "0, 0, 0" "1.000000,1.000000,1.000000") "Undefined" "MultiplyWithRoot" 0 (Utilities|Struct|MakeSTR_Param "NewEnumerator3" 5 0 false (.Index (Utilities|Struct|BreakSTR_CardPosition (Variables|Default|GetFrameCard)))) false self (Variables|Default|GetIDSetter) 0))
        (Transformation|AttachComponentToComponent _returnvalue (Variables|/Game/Blueprints/Map/Board3D/BP_Frame.BP_Frame_C|GetFrame (Variables|Default|GetFrameSelected)) "None" "KeepWorld" "KeepWorld" "KeepWorld" true)
        (Utilities|Array|Add (Variables|Default|GetCardTempArray) _returnvalue)
        (Variables|/Game/Blueprints/Map/Board3D/BP_Frame.BP_Frame_C|SetIsEmpty (Variables|Default|GetFrameSelected) false)
        (Math|Integer|IncrementInt (Variables|Default|GetNbrEnemies)
          (:%20%20
            (Math|Integer|IncrementInt (Variables|Default|GetIDSetter))))))))

(event EventBeginPlay
  (bind _frame (Variables|Default|GetFrame))
  (bind _returnvalue (Transformation|GetWorldLocation _frame))
  (for _index (range 0 4)
    (Variables|Grid|SetI _index)
    (bind _returnvalue_2 (Game|SpawnActorfromClass "/Game/Blueprints/Map/Board3D/BP_Frame.BP_Frame_C" (Math|Transform|MakeTransform (Math|Vector|MakeVector (+ (.x _returnvalue) (Variables|Grid|GetLineDist)) (.y _returnvalue) (.z _returnvalue)) "0, 0, 0" "1.000000,1.000000,1.000000") "Undefined" "MultiplyWithRoot" 0 self 0))
    (bind _output_get (Variables|Grid|SetLineFrame _returnvalue_2))
    (Transformation|AttachActorToActor _output_get self "None" "KeepWorld" "KeepWorld" "KeepWorld" true)
    (Variables|/Game/Blueprints/Map/Board3D/BP_Frame.BP_Frame_C|SetPosition (Variables|Grid|GetLineFrame) (Utilities|Struct|MakeIntPoint (Variables|Grid|GetI) (Variables|Grid|GetJ)))
    (Variables|Grid|SetLineDist (+ (Variables|Grid|GetLineDist) 1e+03))
    (Variables|Grid|SetColumnDist 1e+03)
    (for _index_2 (range 0 5)
      (Variables|Grid|SetJ _index_2)
      (bind _returnvalue_3 (Game|SpawnActorfromClass "/Game/Blueprints/Map/Board3D/BP_Frame.BP_Frame_C" (Math|Transform|MakeTransform (Math|Vector|MakeVector (.x (Transformation|GetWorldLocation (Variables|/Game/Blueprints/Map/Board3D/BP_Frame.BP_Frame_C|GetFrame (Variables|Grid|GetLineFrame)))) (+ (.y (Transformation|GetWorldLocation (Variables|/Game/Blueprints/Map/Board3D/BP_Frame.BP_Frame_C|GetFrame (Variables|Grid|GetLineFrame)))) (Variables|Grid|GetColumnDist)) (.z (Transformation|GetWorldLocation (Variables|/Game/Blueprints/Map/Board3D/BP_Frame.BP_Frame_C|GetFrame (Variables|Grid|GetLineFrame))))) "0, 0, 0" "1.000000,1.000000,1.000000") "Undefined" "MultiplyWithRoot" 0 self 0))
      (bind _output_get_2 (Variables|Grid|SetColumnFrame _returnvalue_3))
      (Transformation|AttachActorToActor _output_get_2 self "None" "KeepWorld" "KeepWorld" "KeepWorld" true)
      (Variables|Grid|SetColumnDist (+ (Variables|Grid|GetColumnDist) 1e+03))
      (Utilities|Map|Add (Variables|Grid|GetGridIndex) (Utilities|Struct|MakeIntPoint (Variables|Grid|GetI) (Variables|Grid|GetJ)) (Utilities|Struct|MakeSTR_CardPosition 0 (Utilities|Struct|MakeIntPoint (Variables|Grid|GetI) (Variables|Grid|GetJ)) (Variables|Grid|GetColumnFrame)))
      (Variables|/Game/Blueprints/Map/Board3D/BP_Frame.BP_Frame_C|SetPosition (Variables|Grid|GetColumnFrame) (Utilities|Struct|MakeIntPoint (Variables|Grid|GetI) (Variables|Grid|GetJ)))))
  (CallFunction|AddCards)
  (Variables|Default|SetGridSize (Utilities|Struct|MakeIntPoint (Variables|Grid|GetI) (Variables|Grid|GetJ))))

(event EventTick
  (params (DeltaSeconds :type Float%20%28single-precision%29))
  (bind _keys (Utilities|Map|Keys (Variables|Grid|GetGridIndex)))
  (for _array_element _keys
    (Development|PrintString (Utilities|String|ToString(Integer) _array_element) true true "(R=0.000000,G=0.052002,B=0.177083,A=1.000000)" 0.0)))

(fn ConstructionScript)