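; Board frame actor for the 3D board map, whose texture shows a status such as ally, enemy, movement, trap or reset.
; SetColor swaps the texture on a dynamic material instance created at BeginPlay.
; Every Tick it traces under the cursor; when hit, it prints its position and highlights as Movement if its grid Y index exceeds 2.
; A hit on another actor resets the highlight.
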(event Custom|SetColor
  (params (Statut :type E_FrameStatut%20Enum :default "NewEnumerator0"))
  (bind _output_get (Variables|Default|SetFrameStatut Statut))
  (Rendering|Material|SetTextureParameterValue (Variables|Default|GetMaterialInstanceFrame) "Frame" (Utilities|Select :Index _output_get :NewEnumerator0 "/Game/Textures/GreenFrame.GreenFrame" :NewEnumerator1 "/Game/Textures/RedFrame.RedFrame" :NewEnumerator2 "/Game/Textures/YellowFrame.YellowFrame" :NewEnumerator3 "/Game/Textures/CardFrame.CardFrame" :NewEnumerator4 "/Game/Textures/BlueFrame.BlueFrame")))

(event EventBeginPlay
  (bind _frame (Variables|Default|GetFrame))
  (bind _asbp_player_controller (Utilities|Casting|CastToBP_PlayerController (Game|GetPlayerController 0)))
  (Variables|Default|SetControllerRef _asbp_player_controller)
  (bind _returnvalue (Rendering|Material|CreateDynamicMaterialInstance _frame 0 (Rendering|Material|GetMaterial _frame 0) "None" :!class /Script/Engine.PrimitiveComponent))
  (Variables|Default|SetMaterialInstanceFrame _returnvalue))

(event Collision|EventActorBeginOverlap
  (params (OtherActor :type Actor%20Object%20Reference)))

(event EventTick
  (params (DeltaSeconds :type Float%20%28single-precision%29))
  (bind _array (Utilities|Array|MakeArray "ObjectTypeQuery2"))
  (bind _controllerref (Variables|Default|GetControllerRef))
  (bind _gridref (Variables|Default|GetGridRef))
  (bind (_hitresult _returnvalue) (Class|PlayerController|GetHitResultUnderCursorforObjects _controllerref _array true))
  (bind _gridindex (Variables|/Game/Blueprints/Map/Board3D/BP_Battle.BP_Battle_C|GetGridIndex _gridref))
  (if _returnvalue
    (if (== (.HitActor (Collision|BreakHitResult _hitresult)) self)
      (Development|PrintString (Utilities|String|ToString(Integer) (Variables|Default|GetPosition)) true true "(R=1.000000,G=0.000000,B=0.056108,A=1.000000)" 0.0)
      (bind _keys (Utilities|Map|Keys _gridindex))
      (for _array_element _keys
        (if (.ReturnValue (Utilities|Map|Find _gridindex _array_element))
          (if (== self (.Frame (Utilities|Struct|BreakSTR_CardPosition (.Value (Utilities|Map|Find _gridindex _array_element)))))
            (if (> (.y (.Index (Utilities|Struct|BreakSTR_CardPosition (.Value (Utilities|Map|Find _gridindex _array_element))))) 2)
              (Variables|Default|SetFrameHovered (.Frame (Utilities|Struct|BreakSTR_CardPosition (.Value (Utilities|Map|Find _gridindex _array_element)))))
              (CallFunction|SetColor "NewEnumerator2")))))
      (else
        (bind _framehovered (Variables|Default|GetFrameHovered)
          (:then
            (CallFunction|SetColor _framehovered "NewEnumerator3")
            (Variables|Default|SetFrameHovered 0))
          (:else))))))

(fn ConstructionScript)