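; BP_pivot is a pivot actor in the MarioUI project that rotates to turn the camera toward a chosen kingdom.
; On BeginPlay it caches every BP_Kingdom actor in an array.
; TurnCamera plays a timeline that lerps the pivot's current rotation toward the look-at rotation from the indexed kingdom to the pivot.
; The lerp restarts from the live rotation on each update, so the turn compounds rather than following the timeline curve directly.
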(event Custom|TurnCamera
  (params (Index :type Integer))
  (bind _alpha (Timeline|Timeline PlayFromStart)
    (:Update
      (Transformation|SetActorRotation (Math|Rotator|Lerp(Rotator) (Transformation|GetActorRotation) (Math|Rotator|FindLookatRotation (Transformation|GetActorLocation (Utilities|Array|Get(acopy) (Variables|Default|GetKingdomRef) Index)) (Transformation|GetActorLocation)) _alpha)))))

(event EventBeginPlay
  (bind _outactors (Actor|GetAllActorsOfClass "/Game/Projects/MarioUI/BP_Kingdom.BP_Kingdom_C"))
  (Variables|Default|SetKingdomRef _outactors))

(event Collision|EventActorBeginOverlap
  (params (OtherActor :type Actor%20Object%20Reference)))

(event EventTick
  (params (DeltaSeconds :type Float%20%28single-precision%29)))

(fn ConstructionScript)